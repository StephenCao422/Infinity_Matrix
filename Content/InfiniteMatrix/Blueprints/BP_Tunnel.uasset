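; Endless tunnel segment with a rotating holed wall, optional health pickup and enemy.
; Player overlap with TriggerZone adds score, asks TunnelSpawner for another tunnel and destroys this one.
; Overlaps apply wall damage with death check, change player health via visible pickup or enemy, or destroy the enemy for score on non-player contact.
; Uncalled-here functions randomize wall mesh and roll, and chance-based pickup and enemy placement.
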(event `self.ReceiveTick`
  (params (DeltaSeconds :type "Float (single-precision)"))
  (`SceneComponent.K2_AddLocalRotation` (`self.WallMesh`) (`KismetMathLibrary.MakeRotator` (* DeltaSeconds (`self.RotateSpeed`))) false false))

(event `self.TriggerZone.OnComponentBeginOverlap`
  (params (OverlappedComponent :type "PrimitiveComponent Object Reference") (OtherActor :type "Actor Object Reference") (OtherComp :type "PrimitiveComponent Object Reference") (OtherBodyIndex :type Integer) (bFromSweep :type Boolean) (SweepResult :type "HitResult Structure (by ref)"))
  (bind _asbp_player (cast `/Game/InfiniteMatrix/Blueprints/BP_Player` OtherActor))
  (`/Game/InfiniteMatrix/Blueprints/BP_Player.ChangeScore` _asbp_player)
  (`/Game/InfiniteMatrix/Blueprints/BP_TunnelSpawner.SpawnTunnelAtSpawnPoint` (`self.TunnelSpawner`))
  (`self.K2_DestroyActor`))

(event `self.WallMesh.OnComponentBeginOverlap`
  (params (OverlappedComponent :type "PrimitiveComponent Object Reference") (OtherActor :type "Actor Object Reference") (OtherComp :type "PrimitiveComponent Object Reference") (OtherBodyIndex :type Integer) (bFromSweep :type Boolean) (SweepResult :type "HitResult Structure (by ref)"))
  (`GameplayStatics.ApplyDamage` OtherActor -10.0)
  (bind _asbp_player (cast `/Game/InfiniteMatrix/Blueprints/BP_Player` OtherActor))
  (set `/Game/InfiniteMatrix/Blueprints/BP_Player.WallHit` true _asbp_player)
  (`/Engine/EditorBlueprintResources/StandardMacros.CompareFloat` (`/Game/InfiniteMatrix/Blueprints/BP_Player.Health` _asbp_player) 1.0
    (:`<`
      (set `/Game/InfiniteMatrix/Blueprints/BP_Player.IsDead` true _asbp_player)
      (`/Game/InfiniteMatrix/Blueprints/BP_Player.DisplayRestart` _asbp_player))))

(event `self.HealthPackage.OnComponentBeginOverlap`
  (params (OverlappedComponent :type "PrimitiveComponent Object Reference") (OtherActor :type "Actor Object Reference") (OtherComp :type "PrimitiveComponent Object Reference") (OtherBodyIndex :type Integer) (bFromSweep :type Boolean) (SweepResult :type "HitResult Structure (by ref)"))
  (bind _asbp_player (cast `/Game/InfiniteMatrix/Blueprints/BP_Player` OtherActor))
  (if (`SceneComponent.IsVisible` (`self.HealthPackage`))
    (set `/Game/InfiniteMatrix/Blueprints/BP_Player.Health` (+ (`/Game/InfiniteMatrix/Blueprints/BP_Player.Health` _asbp_player) 10.0) _asbp_player)))

(event `self.Enemy.OnComponentBeginOverlap`
  (params (OverlappedComponent :type "PrimitiveComponent Object Reference") (OtherActor :type "Actor Object Reference") (OtherComp :type "PrimitiveComponent Object Reference") (OtherBodyIndex :type Integer) (bFromSweep :type Boolean) (SweepResult :type "HitResult Structure (by ref)"))
  (if (== (`GameplayStatics.GetObjectClass` OtherActor) "/Game/InfiniteMatrix/Blueprints/BP_Player.BP_Player_C")
    (bind _asbp_player (cast `/Game/InfiniteMatrix/Blueprints/BP_Player` OtherActor))
    (if (`SceneComponent.IsVisible` (`self.Enemy`))
      (set `/Game/InfiniteMatrix/Blueprints/BP_Player.Health` (`KismetMathLibrary.FClamp` (- (`/Game/InfiniteMatrix/Blueprints/BP_Player.Health` _asbp_player) 10.0) 0.0 100.0) _asbp_player))
    (else
      (`ActorComponent.K2_DestroyComponent` (`self.Enemy`))
      (bind _returnvalue (`GameplayStatics.GetActorOfClass` "/Game/InfiniteMatrix/Blueprints/BP_Player.BP_Player_C"))
      (`/Game/InfiniteMatrix/Blueprints/BP_Player.ChangeScore` _returnvalue))))

(fn `RandomEnemy`
  (bind _enemy (`self.Enemy`))
  (bind _enemy_2 (`self.Enemy`))
  (`/Engine/EditorBlueprintResources/StandardMacros.CompareInt` (`KismetMathLibrary.RandomIntegerInRange` 0 1) 1
    (:`==`
      (if true
        (`SceneComponent.K2_AddLocalOffset` (`self.Enemy`) (`KismetMathLibrary.MakeVector` (`KismetMathLibrary.RandomFloatInRange` -200.0 200.0) (`KismetMathLibrary.RandomFloatInRange` -200.0 200.0) (`KismetMathLibrary.RandomFloatInRange` -200.0 200.0)) false false)
        (`SceneComponent.SetHiddenInGame` _enemy false false)
        (`PrimitiveComponent.SetCollisionEnabled` _enemy_2 "QueryAndPhysics")
        (else
          (`SceneComponent.SetHiddenInGame` _enemy false false)
          (`PrimitiveComponent.SetCollisionEnabled` _enemy_2 "NoCollision"))))))

(fn `RandomizeGPackage`
  (bind _healthpackage (`self.HealthPackage`))
  (bind _healthpackage_2 (`self.HealthPackage`))
  (`/Engine/EditorBlueprintResources/StandardMacros.CompareInt` (`KismetMathLibrary.RandomIntegerInRange` 0 9)
    (:`==`
      (if true
        (`SceneComponent.K2_AddLocalOffset` (`self.HealthPackage`) (`KismetMathLibrary.MakeVector` (`KismetMathLibrary.RandomFloatInRange` -200.0 200.0) (`KismetMathLibrary.RandomFloatInRange` -200.0 200.0) (`KismetMathLibrary.RandomFloatInRange` -200.0 200.0)) false false)
        (`SceneComponent.SetHiddenInGame` _healthpackage false false)
        (`PrimitiveComponent.SetCollisionEnabled` _healthpackage_2 "QueryAndPhysics")
        (else
          (`SceneComponent.SetHiddenInGame` _healthpackage true false)
          (`PrimitiveComponent.SetCollisionEnabled` _healthpackage_2 "NoCollision"))))))

(fn `RandomizeWall`
  (`StaticMeshComponent.SetStaticMesh` (`self.WallMesh`) (select `int` (`KismetMathLibrary.RandomIntegerInRange` 0 3) :`0` "/Game/InfiniteMatrix/Meshes/SM_Hole_01.SM_Hole_01" :`1` "/Game/InfiniteMatrix/Meshes/SM_Hole_02.SM_Hole_02" :`2` "/Game/InfiniteMatrix/Meshes/SM_Hole_03.SM_Hole_03" :`3` "/Game/InfiniteMatrix/Meshes/SM_Hole_04.SM_Hole_04" :!type "StaticMesh Object Reference"))
  (`SceneComponent.K2_AddLocalRotation` (`self.WallMesh`) (`KismetMathLibrary.MakeRotator` (`KismetMathLibrary.RandomFloatInRange` 0.0 360.0)) false false))

(fn `UserConstructionScript`)